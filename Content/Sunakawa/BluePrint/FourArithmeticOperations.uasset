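; Blueprint that generates random four-operation arithmetic questions for the game, storing them in the GameJamInstance.
; Tick polls the instance's UpdateFlg, which ON_UpdateFlg sets; when true, it rolls two single-digit operands, calls ForrArithmeticOperations, then clears the flag.
; That function randomly picks add, subtract, multiply or divide and writes the operator symbol and answer back to the instance.
; Division has no guard against a zero divisor or uneven results.
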(event `self.ReceiveBeginPlay`
  ;[1 1 1] ゲームインスタンスの参照を持つ
  (bind _asgame_jam_instance (cast `/Game/Sunakawa/BluePrint/GameJamInstance` (`GameplayStatics.GetGameInstance`)))
  (set `self.GameJamInstance` _asgame_jam_instance))

(event `self.ReceiveTick`
  (params (DeltaSeconds :type "Float (single-precision)"))
  (bind _returnvalue (`KismetMathLibrary.RandomIntegerInRange` 0 9))
  (bind _gamejaminstance (`self.GameJamInstance`))
  ;[1 1 1] 計算する値の更新
  (if (`/Game/Sunakawa/BluePrint/GameJamInstance.UpdateFlg` _gamejaminstance)
    (set `/Game/Sunakawa/BluePrint/GameJamInstance.Value_A` _returnvalue _gamejaminstance)
    (set `/Game/Sunakawa/BluePrint/GameJamInstance.Value_B` _returnvalue _gamejaminstance)
    (`self.ForrArithmeticOperations`)
    (set `/Game/Sunakawa/BluePrint/GameJamInstance.UpdateFlg` false _gamejaminstance)))

(event `ON_UpdateFlg`
  ;[1 1 1] 演算子を更新するフラグをTrueにする
  (set `/Game/Sunakawa/BluePrint/GameJamInstance.UpdateFlg` true (`self.GameJamInstance`)))

(fn `ForrArithmeticOperations`
  (locals (A :type Integer) (B :type Integer))
  (bind _gamejaminstance (`self.GameJamInstance`))
  (bind _gamejaminstance_2 (`self.GameJamInstance`))
  (bind _gamejaminstance_3 (`self.GameJamInstance`))
  (set `local.A` (`/Game/Sunakawa/BluePrint/GameJamInstance.Value_A` _gamejaminstance_3))
  (set `local.B` (`/Game/Sunakawa/BluePrint/GameJamInstance.Value_B` _gamejaminstance_3))
  (switch `int` (`KismetMathLibrary.RandomIntegerInRange` 0 3)
    (:`0`
      (set `/Game/Sunakawa/BluePrint/GameJamInstance.Operator` "+" _gamejaminstance)
      (set `/Game/Sunakawa/BluePrint/GameJamInstance.Answer` (+ (`local.A`) (`local.B`)) _gamejaminstance_2))
    (:`1`
      (set `/Game/Sunakawa/BluePrint/GameJamInstance.Operator` "-" _gamejaminstance)
      (set `/Game/Sunakawa/BluePrint/GameJamInstance.Answer` (- (`local.A`) (`local.B`)) _gamejaminstance_2))
    (:`2`
      (set `/Game/Sunakawa/BluePrint/GameJamInstance.Operator` "×" _gamejaminstance)
      (set `/Game/Sunakawa/BluePrint/GameJamInstance.Answer` (* (`local.A`) (`local.B`)) _gamejaminstance_2))
    (:`3`
      (set `/Game/Sunakawa/BluePrint/GameJamInstance.Operator` "÷" _gamejaminstance)
      (set `/Game/Sunakawa/BluePrint/GameJamInstance.Answer` (/ (`local.A`) (`local.B`)) _gamejaminstance_2))))

(fn `UserConstructionScript`)